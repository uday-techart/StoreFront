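; BP_Storefront is a configurable storefront prop whose mesh and surface look are set through Blueprint variables.
; Its construction script assigns the chosen mesh and creates a dynamic material instance from a parent material.
; It pushes tiling, offset, roughness, normal map and glow map variables into that instance as scalar parameters, then applies it to material slot 0.
; The event graph holds only disabled default events, so no gameplay logic runs.
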(fn `UserConstructionScript`
  (`StaticMeshComponent.SetStaticMesh` (`self.StaticMesh`) (`self.Mesh`))
  (bind _returnvalue (`KismetMaterialLibrary.CreateDynamicMaterialInstance` (`self.MaterialInstance`)))
  (bind _output_get (set `self.MID` _returnvalue))
  (`MaterialInstanceDynamic.SetScalarParameterValue` _output_get "U-Tiling" (`self.UTiling`))
  (`MaterialInstanceDynamic.SetScalarParameterValue` (`self.MID`) "V-Tiling" (`self.VTiling`))
  (`MaterialInstanceDynamic.SetScalarParameterValue` (`self.MID`) "U-Offset" (`self.U-Offset`))
  (`MaterialInstanceDynamic.SetScalarParameterValue` (`self.MID`) "V-Offset" (`self.V-Offset`))
  (`MaterialInstanceDynamic.SetScalarParameterValue` (`self.MID`) "Roughness Min" (`self.RoughnessMin`))
  (`MaterialInstanceDynamic.SetScalarParameterValue` (`self.MID`) "Roughness Max" (`self.RoughnessMax`))
  (`MaterialInstanceDynamic.SetScalarParameterValue` (`self.MID`) "NormalMap Tiling" (`self.NormalMapTiling`))
  (`MaterialInstanceDynamic.SetScalarParameterValue` (`self.MID`) "Flatten Intensity" (`self.NormalMap Intensity`))
  (`MaterialInstanceDynamic.SetScalarParameterValue` (`self.MID`) "GlowMap Offset" (`self.GlowMapOffset`))
  (`MaterialInstanceDynamic.SetScalarParameterValue` (`self.MID`) "GlowMap Contrast" (`self.GlowMapContrast`))
  (`PrimitiveComponent.SetMaterial` (`self.StaticMesh`) 0 (`self.MID`)))